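; Fireball projectile actor that flies to a target and removes itself on arrival.
; On BeginPlay it caches all ProjectileTarget_BP actors and uses the first one as its destination.
; Tick moves the root at constant speed, without sweeping, toward a point slightly above that target's static mesh.
; When the positions match, it deactivates the Fireball effect and destroys itself after a short delay.
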(event EventBeginPlay
  (bind _outactors (Actor|GetAllActorsOfClass "/Game/VFXapprentice/Joppa/Fireball/ProjectileTarget_BP.ProjectileTarget_BP_C")))

(event EventTick
  (params (DeltaSeconds :type Float%20%28single-precision%29))
  (bind _defaultsceneroot (Variables|Default|GetDefaultSceneRoot))
  (bind _returnvalue (Transformation|GetWorldLocation _defaultsceneroot))
  (Transformation|SetWorldLocation (Variables|Default|GetDefaultSceneRoot) (Math|Interpolation|VInterptoConstant _returnvalue (+ (Transformation|GetWorldLocation (Variables|/Script/Engine.StaticMeshActor|GetStaticMeshComponent (Utilities|Array|Get(acopy) (stale EventBeginPlay _outactors)))) "0, 0,35.000000") (Math|Float|Fraction DeltaSeconds) 1e+03) false false)
  (if (Math|Vector|Equal(Vector) _returnvalue (+ (Transformation|GetWorldLocation (Variables|/Script/Engine.StaticMeshActor|GetStaticMeshComponent (Utilities|Array|Get(acopy) (stale EventBeginPlay _outactors)))) "0, 0,35.000000") 0.0001)
    (Components|Activation|Deactivate (Variables|Default|GetFireball))
    (Utilities|FlowControl|Delay 1.5)
    (Actor|DestroyActor)))

(fn ConstructionScript)